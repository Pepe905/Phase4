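; Player controller for the Phase 4 multiplayer match, managing the local player's UI and saved profile.
; On BeginPlay the local controller builds the in-game HUD and chest prompt, then loads the profile save, sending it to the server when remote.
; On possession it hands both widgets to the pawn; Tick shows the chest prompt while the pawn is inside a box collider.
; It also handles profile saving, countdown, death menu and leaving the session.
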(event Custom|EnableAllInput
  (Input|EnableInput (Pawn|GetControlledPawn) self))

(event Custom|GameStartCountdown
  (Default|GameStartCountdown (Variables|Default|GetWB_Countdown)))

(event Custom|UnHide_IngameHUD
  (Widget|SetVisibility (Variables|Default|GetWB_Countdown) "Visible"))

(event Custom|EndClientSession
  (bind _asbp_phase_4_gameinstance (Utilities|Casting|CastToBP_Phase4_Gameinstance (Game|GetGameInstance)))
  (Variables|/Game/Framework/BP_Phase4_Gameinstance.BP_Phase4_Gameinstance_C|SetMP_IsPauseMenuVisible _asbp_phase_4_gameinstance false)
  (|DestroySession self
    (:then
      (Game|OpenLevel(byName) "MainMenu_Placeholder"))))

(event Custom|Local_SetHUDVar
  (bind _wb_countdown (Variables|Default|GetWB_Countdown))
  (Utilities|FlowControl|Delay 0.5)
  (bind _ascharacter_prototype_2_base (Utilities|Casting|CastToCharacter_Prototype_2_Base (Pawn|GetControlledPawn)))
  (Variables|/Game/Assets/Character/Character_Prototype_2_Base.Character_Prototype_2_Base_C|SetInGame_HUD _ascharacter_prototype_2_base _wb_countdown)
  (Variables|/Game/Assets/Character/Character_Prototype_2_Base.Character_Prototype_2_Base_C|SetNewVar_0 _ascharacter_prototype_2_base 0)
  (Variables|/Game/Assets/Character/Character_Prototype_2_Base.Character_Prototype_2_Base_C|SetNew%20Var%206 _ascharacter_prototype_2_base (Variables|Default|GetNewVar_6))
  (Default|UpdateHealth _wb_countdown (Variables|/Game/Assets/Character/Character_Prototype_2_Base.Character_Prototype_2_Base_C|GetHealth _ascharacter_prototype_2_base) false)
  (Default|UpdateShield _wb_countdown (Variables|/Game/Assets/Character/Character_Prototype_2_Base.Character_Prototype_2_Base_C|GetShield _ascharacter_prototype_2_base) false))

(event Custom|Svr_SetPlayerProfile
  (params (Player%20Profile :type S%20Player%20Profile%20Structure))
  (Variables|Default|SetPlayer%20Profile Player%20Profile))

(event Custom|Save_CareerXpandLevel
  (bind _as_sg_player_profile (Variables|Default|GetAs%20SG%20Player%20Profile))
  (Utilities|FlowControl|RetriggerableDelay 0.5)
  (Variables|/Game/SavedData/SG_PlayerProfile.SG_PlayerProfile_C|SetPlayerProfile _as_sg_player_profile (Variables|Default|GetPlayer%20Profile))
  (SaveGame|SaveGametoSlot _as_sg_player_profile "PlayerProfile_Slot"))

(event EventBeginPlay
  (if (Pawn|IsLocalPlayerController)
    (Viewport|RemoveAllWidgets)
    (CallFunction|UIShowIngameHUD)
    (Input|SetInputModeGameOnly self)
    (Variables|Default|SetbShowMouseCursor false)
    (bind _returnvalue (SaveGame|LoadGamefromSlot "PlayerProfile_Slot"))
    (bind _assg_player_profile (Utilities|Casting|CastToSG_PlayerProfile _returnvalue))
    (Variables|Default|SetAs%20SG%20Player%20Profile _assg_player_profile)
    (Networking|SwitchHasAuthority
      (:Authority
        (Variables|Default|SetPlayer%20Profile (Variables|/Game/SavedData/SG_PlayerProfile.SG_PlayerProfile_C|GetPlayerProfile _assg_player_profile)))
      (:Remote
        (CallFunction|SvrSetPlayerProfile (Variables|/Game/SavedData/SG_PlayerProfile.SG_PlayerProfile_C|GetPlayerProfile _assg_player_profile))))))

(event EventTick
  (params (DeltaSeconds :type Float%20%28single-precision%29))
  (Utilities|FlowControl|Sequence
    (:then_0
      (bind _ascharacter_prototype_2_base (Utilities|Casting|CastToCharacter_Prototype_2_Base (Pawn|GetControlledPawn)))
      (if (Variables|/Game/Assets/Character/Character_Prototype_2_Base.Character_Prototype_2_Base_C|GetisInsideBoxCollider _ascharacter_prototype_2_base)
        (Widget|SetVisibility (Variables|Default|GetNewVar_6) "Visible")
        (else
          (Widget|SetVisibility (Variables|Default|GetNewVar_6) "Hidden"))))))

(event EventPossess
  (params (PossessedPawn :type Pawn%20Object%20Reference))
  (CallFunction|LocalSetHUDVar))

(fn ConstructionScript)

(fn UIShowIngameHUD
  (Utilities|IsValid (Variables|Default|GetWB_Countdown)
    (:Is%20Valid
      (UserInterface|Viewport|AddtoViewport (Variables|Default|GetWB_Countdown) 0 :!label _label))
    (:Is%20Not%20Valid
      (Utilities|FlowControl|Sequence
        (:then_6
          (bind _returnvalue (UserInterface|CreateWidget "/Game/UI/HUD/ChestOpen_Widget.ChestOpen_Widget_C" self))
          (bind _output_get (Variables|Default|SetNewVar_6 _returnvalue))
          (UserInterface|Viewport|AddtoViewport _output_get 0)
          (Widget|SetVisibility (Variables|Default|GetNewVar_6) "Hidden"))
        (:then_7
          (bind _returnvalue_2 (UserInterface|CreateWidget "/Game/UI/HUD/InGame_HUD_Widget.InGame_HUD_Widget_C" self))
          (Variables|Default|SetWB_Countdown _returnvalue_2)
          (goto _label))))))

(fn UIShowPlayerDied
  (Utilities|IsValid (Variables|Default|GetWB_PlayerDied)
    (:Is%20Valid
      _)
    (:Is%20Not%20Valid
      (bind _returnvalue (UserInterface|CreateWidget "/Game/Assets/Map/Menu/MenuWidgets/WB_PlayerDiedMenu.WB_PlayerDiedMenu_C" self))
      (Variables|Default|SetWB_PlayerDied _returnvalue)))
  (UserInterface|Viewport|AddtoViewport (Variables|Default|GetWB_PlayerDied) 0)
  (Input|SetInputModeUIOnly self 0 "DoNotLock")
  (Variables|Default|SetbShowMouseCursor true)
  (return))