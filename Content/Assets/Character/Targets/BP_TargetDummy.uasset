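; BP_TargetDummy is a target dummy with a skeletal mesh and capsule that removes itself when hit while ragdolled.
; On Hit, if the mesh is simulating physics, it applies a zero-strength impulse at the actor's location and immediately destroys the actor; otherwise nothing happens.
; The construction script holds only a disconnected debug print that computes the mesh's relative Z offset from the capsule half-height.
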(event Collision|EventHit
  (params (MyComp :type Primitive%20Component%20Object%20Reference) (Other :type Actor%20Object%20Reference) (OtherComp :type Primitive%20Component%20Object%20Reference) (bSelfMoved :type Boolean) (HitLocation :type Vector :default "0, 0, 0") (HitNormal :type Vector :default "0, 0, 0") (NormalImpulse :type Vector :default "0, 0, 0") (Hit :type Hit%20Result%20Structure%20%28by%20ref%29))
  (if (Physics|IsSimulatingPhysics (Variables|Character|GetMesh) "None")
    (Physics|AddImpulseatLocation (Variables|Character|GetMesh) "0, 0, 0" (Transformation|GetActorLocation) "None")
    (Actor|DestroyActor)))

(fn ConstructionScript)