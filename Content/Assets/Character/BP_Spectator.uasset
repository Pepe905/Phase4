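; BP_Spectator is a spectator pawn that follows living players, destroying itself when unpossessed.
; On possession it shows spectator controls, gathers all Character_Prototype_2_Base actors and attaches to a living one.
; Left/Right refresh the player list and cycle with wraparound through Svr-prefixed events, skipping dead players via a delayed retry loop.
; Each switch snaps the pawn to the target and updates the spectated name on the HUD.
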(event Custom|Svr_AttachToPlayer
  (params (IncreaseIndex :type Boolean))
  (if IncreaseIndex
    (Math|Integer|IncrementInt (Variables|Default|GetCurrentPlayerIndex) :!label _label
      (:%20%20
        (if (== (Variables|Default|GetCurrentPlayerIndex) (Utilities|Array|Length (Variables|Default|GetAllPlayers)))
          (Variables|Default|SetCurrentPlayerIndex 0))
        (if (Variables|/Game/Assets/Character/Character_Prototype_2_Base.Character_Prototype_2_Base_C|GetisAlive (Utilities|Array|Get(acopy) (Variables|Default|GetAllPlayers) (Variables|Default|GetCurrentPlayerIndex)))
          (Variables|Default|SetAttachedPlayer (Utilities|Array|Get(acopy) (Variables|Default|GetAllPlayers) (Variables|Default|GetCurrentPlayerIndex)))
          (Transformation|AttachActorToActor (Variables|Default|GetAttachedPlayer) "None" "SnapToTarget" "SnapToTarget" "KeepRelative" true :!label _label_2)
          (Default|UpdateHUDSpecPlayerName (Variables|Default|GetAs%20BP%20Phase%204%20Player%20Controller) (.playername (Variables|/Game/Framework/BP_Phase4_PlayerController.BP_Phase4_PlayerController_C|GetPlayer%20Profile (Variables|/Game/Assets/Character/Character_Prototype_2_Base.Character_Prototype_2_Base_C|GetPhase4PlayerController (Variables|Default|GetAttachedPlayer)))))
          (elif (> (Utilities|Array|Length (Variables|Default|GetAllPlayers)) 1)
            (Utilities|FlowControl|Delay 0.1)
            (goto _label)))))
    (else
      (Math|Integer|DecrementInt (Variables|Default|GetCurrentPlayerIndex) :!label _label_3
        (:%20%20
          (if (< (Variables|Default|GetCurrentPlayerIndex) 0)
            (Variables|Default|SetCurrentPlayerIndex (- (Utilities|Array|Length (Variables|Default|GetAllPlayers)) 1)))
          (if (Variables|/Game/Assets/Character/Character_Prototype_2_Base.Character_Prototype_2_Base_C|GetisAlive (Utilities|Array|Get(acopy) (Variables|Default|GetAllPlayers) (Variables|Default|GetCurrentPlayerIndex)))
            (Variables|Default|SetAttachedPlayer (Utilities|Array|Get(acopy) (Variables|Default|GetAllPlayers) (Variables|Default|GetCurrentPlayerIndex)))
            (goto _label_2)
            (elif (> (Utilities|Array|Length (Variables|Default|GetAllPlayers)) 1)
              (Utilities|FlowControl|Delay 0.1)
              (goto _label_3))))))))

(event Custom|Svr_UpdatePlayers
  (bind _arrayelement (Utilities|Array|ReverseforEachLoop (Variables|Default|GetAllPlayers))
    (:LoopBody
      (Utilities|IsValid _arrayelement
        (:Is%20Valid
          (Utilities|Array|RemoveItem (Variables|Default|GetAllPlayers) _arrayelement))))
    (:Completed
      (bind _outactors (Actor|GetAllActorsOfClass "/Game/Assets/Character/Character_Prototype_2_Base.Character_Prototype_2_Base_C"))
      (for _array_element _outactors
        (Utilities|Array|AddUnique (Variables|Default|GetAllPlayers) _array_element)
        (Utilities|IsValid (Variables|Default|GetAttachedPlayer)
          (:Is%20Valid
            (Variables|Default|SetCurrentPlayerIndex (Utilities|Array|FindItem (Variables|Default|GetAllPlayers) (Variables|Default|GetAttachedPlayer)))))))))

(event EventPossessed
  (params (NewController :type Controller%20Object%20Reference))
  (bind _asbp_phase_4_player_controller (Utilities|Casting|CastToBP_Phase4_PlayerController NewController))
  (bind _output_get (Variables|Default|SetAs%20BP%20Phase%204%20Player%20Controller _asbp_phase_4_player_controller))
  (Default|ShowSpectatorControls _output_get)
  (bind _outactors (Actor|GetAllActorsOfClass "/Game/Assets/Character/Character_Prototype_2_Base.Character_Prototype_2_Base_C"))
  (Variables|Default|SetAllPlayers _outactors)
  (CallFunction|SvrAttachtoPlayer true))

(event EventUnpossessed
  (params (OldController :type Controller%20Object%20Reference))
  (Actor|DestroyActor))

(event Input|ActionEvents|InputActionPauseGame
  (params (Key :type Key%20Structure :default "None"))
  (:Pressed
    (bind _asbp_phase_4_gameinstance (Utilities|Casting|CastToBP_Phase4_Gameinstance (Game|GetGameInstance)))
    (Default|TogglePauseGame _asbp_phase_4_gameinstance)))

(event Input|AxisEvents|InputAxisLookUp
  (params (AxisValue :type Float%20%28single-precision%29))
  (Pawn|Input|AddControllerPitchInput AxisValue))

(event Input|KeyboardEvents|Right
  (params (Key :type Key%20Structure :default "None"))
  (:Pressed
    (CallFunction|SvrUpdatePlayers)
    (CallFunction|SvrAttachtoPlayer true)))

(event Input|KeyboardEvents|Left
  (params (Key :type Key%20Structure :default "None"))
  (:Pressed
    (CallFunction|SvrUpdatePlayers)
    (CallFunction|SvrAttachtoPlayer false)))

(fn ConstructionScript)