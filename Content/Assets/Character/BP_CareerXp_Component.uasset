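; Character component that tracks a player's career XP and level, capped at level 10.
; On init it loads the XP threshold map, reads the profile from player controller 0, then refreshes the countdown widget and saves.
; Added XP runs on server or owning client, can skip several levels, and rewrites the controller's profile with a hardcoded character choice.
; Only the locally controlled character refreshes the HUD and saves.
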(event Custom|CareerXp_Component_Init
  (CallFunction|SetupCareerXpMap)
  (bind _ascharacter_prototype_2_base (Utilities|Casting|CastToCharacter_Prototype_2_Base (Components|GetOwner)))
  (Variables|Default|SetAs%20Character%20Prototype%202 _ascharacter_prototype_2_base)
  (bind _asbp_phase_4_player_controller (Utilities|Casting|CastToBP_Phase4_PlayerController (Game|GetPlayerController 0)))
  (bind _output_get (Variables|Default|SetAs%20BP%20Phase%204%20Player%20Controller _asbp_phase_4_player_controller))
  (Variables|Default|SetPlayer%20Career%20Xp (.player_career_xp (Variables|/Game/Framework/BP_Phase4_PlayerController.BP_Phase4_PlayerController_C|GetPlayer%20Profile _output_get)))
  (Variables|Default|SetPlayer%20Career%20Level (.player_career_level (Variables|/Game/Framework/BP_Phase4_PlayerController.BP_Phase4_PlayerController_C|GetPlayer%20Profile _output_get)))
  (if (Pawn|IsLocalPlayerController (Variables|Default|GetAs%20BP%20Phase%204%20Player%20Controller))
    (Default|UpdateXpAmount (Variables|/Game/Framework/BP_Phase4_PlayerController.BP_Phase4_PlayerController_C|GetWB_Countdown (Variables|Default|GetAs%20BP%20Phase%204%20Player%20Controller)))
    (Default|UpdateXpLevel (Variables|/Game/Framework/BP_Phase4_PlayerController.BP_Phase4_PlayerController_C|GetWB_Countdown (Variables|Default|GetAs%20BP%20Phase%204%20Player%20Controller)))
    (Default|SaveCareerXpandLevel (Variables|Default|GetAs%20BP%20Phase%204%20Player%20Controller))))

(event Custom|Add_CareerXp
  (params (XpAmount :type Integer))
  (bind _as_character_prototype_2 (Variables|Default|GetAs%20Character%20Prototype%202))
  (bind _ingame_hud (Variables|/Game/Assets/Character/Character_Prototype_2_Base.Character_Prototype_2_Base_C|GetInGame_HUD _as_character_prototype_2))
  (if (or (Networking|IsServer) (Pawn|IsLocallyControlled (Variables|Default|GetAs%20Character%20Prototype%202)))
    (bind _output_get (Variables|Default|SetPlayer%20Career%20Xp (+ (Variables|Default|GetPlayer%20Career%20Xp) XpAmount)))
    (bind (_cancareerlvlup _newcareerlevel) (CallFunction|CheckforRankUp _output_get))
    (if _cancareerlvlup
      (Variables|Default|SetPlayer%20Career%20Level _newcareerlevel))
    (CallFunction|UpdatePlayerControllerProfile)
    (if (Pawn|IsLocallyControlled _as_character_prototype_2)
      (Default|UpdateXpAmount _ingame_hud)
      (Default|UpdateXpLevel _ingame_hud)
      (Default|SaveCareerXpandLevel (Variables|Default|GetAs%20BP%20Phase%204%20Player%20Controller)))))

(fn SetupCareerXpMap
  (Variables|Default|SetCareerXp_Map_Levels (.xp_map_levels (LocalVariables|GetS_XpandLevel)))
  (return))

(fn CheckforRankUp
  (params (CareerXpAmount :type Integer))
  (LocalVariables|SetLcl_CurrentCareerXp CareerXpAmount)
  (LocalVariables|SetLcl_CurrentCareerRank (Variables|Default|GetPlayer%20Career%20Level))
  (if (and (> (LocalVariables|GetLcl_CurrentCareerXp) (Utilities|Array|Get(acopy) (Variables|Default|GetCareerXp_Map_Levels) (LocalVariables|GetLcl_CurrentCareerRank))) (< (LocalVariables|GetLcl_CurrentCareerRank) 10))
    (LocalVariables|SetLcl_CanRankUp true)
    (bind _index (Utilities|FlowControl|ForLoopwithBreak (LocalVariables|GetLcl_CurrentCareerRank) 10 :!label _label)
      (:LoopBody
        (if (not (> (LocalVariables|GetLcl_CurrentCareerXp) (Utilities|Array|Get(acopy) (Variables|Default|GetCareerXp_Map_Levels) _index)))
          (LocalVariables|SetLcl_CurrentCareerRank _index)
          (goto _label Break)))
      (:Completed
        (return (LocalVariables|GetLcl_CanRankUp) (LocalVariables|GetLcl_CurrentCareerRank))))
    (else
      (LocalVariables|SetLcl_CanRankUp false)
      (return (LocalVariables|GetLcl_CanRankUp) (LocalVariables|GetLcl_CurrentCareerRank)))))

(fn UpdatePlayerControllerProfile
  (bind _as_bp_phase_4_player_controller (Variables|Default|GetAs%20BP%20Phase%204%20Player%20Controller))
  (Variables|/Game/Framework/BP_Phase4_PlayerController.BP_Phase4_PlayerController_C|SetPlayer%20Profile _as_bp_phase_4_player_controller (Utilities|Struct|MakeS_PlayerProfile (.playername (Variables|/Game/Framework/BP_Phase4_PlayerController.BP_Phase4_PlayerController_C|GetPlayer%20Profile _as_bp_phase_4_player_controller)) (Variables|Default|GetPlayer%20Career%20Xp) (Variables|Default|GetPlayer%20Career%20Level) "Prototype2_Clean" "/Game/Assets/Character/Character_Prototype_2_Clean.Character_Prototype_2_Clean_C"))
  (return))