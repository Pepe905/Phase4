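; Weapon effects actor that plays Niagara muzzle flash and tracer effects when WeaponFired receives impact positions.
; Reuses each attached system while active, otherwise spawns a new one at the muzzle socket, and toggles User.Trigger per shot.
; The flash receives a direction toward the first impact; the tracer receives the whole impact array.
; A retriggerable delay polls both auto-destroying systems and destroys the actor once neither remains valid.
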(event Custom|WeaponFired
  (params (ImpactPositions :type Array%20of%20Vectors))
  (Variables|Default|SetImpact%20Positions ImpactPositions)
  (Utilities|FlowControl|Sequence
    (:then_0
      (Utilities|IsValid (Variables|Default|GetNS_MuzzleFlash)
        (:Is%20Valid
          (if (Components|Activation|IsActive (Variables|Default|GetNS_MuzzleFlash))
            _
            (else
              (bind _returnvalue (Niagara|SpawnSystemAttached (Variables|Default|GetMuzzleFlashFX) (Variables|Default|GetDefaultSceneRoot) "None" (.location (Transformation|GetSocketTransform (Variables|Default|GetWeaponMesh) (Variables|Default|GetMuzzleSocket) "RTS_Component")) "0.000000,90.000000,0.000000" "KeepRelativeOffset" true :!label _label))
              (Variables|Default|SetNS_MuzzleFlash _returnvalue)
              (Variables|Default|SetMuzzleFlashTrigger false))))
        (:Is%20Not%20Valid
          (goto _label)))
      (Variables|Default|SetMuzzleFlashTrigger (not (Variables|Default|GetMuzzleFlashTrigger)))
      (Niagara|SetNiagaraVariable(Vector3) (Variables|Default|GetNS_MuzzleFlash) "User.Direction" (Math|Vector|Normalize (- (Utilities|Array|Get(acopy) (Variables|Default|GetImpact%20Positions)) (.location (Transformation|GetSocketTransform (Variables|Default|GetWeaponMesh) (Variables|Default|GetMuzzleSocket) "RTS_Component")))))
      (Class|NiagaraComponent|SetVariableBool (Variables|Default|GetNS_MuzzleFlash) "User.Trigger" (Variables|Default|GetMuzzleFlashTrigger)))
    (:then_1
      (Utilities|IsValid (Variables|Default|GetNS_TracerFX)
        (:Is%20Valid
          (if (Components|Activation|IsActive (Variables|Default|GetNS_TracerFX))
            _
            (else
              (bind _returnvalue_2 (Niagara|SpawnSystemAttached (Variables|Default|GetTracerFx) (Variables|Default|GetDefaultSceneRoot) "None" (.location (Transformation|GetSocketTransform (Variables|Default|GetWeaponMesh) (Variables|Default|GetMuzzleSocket) "RTS_Component")) "0.000000,-90.000000,0.000000" "KeepRelativeOffset" true :!label _label_2))
              (Variables|Default|SetNS_TracerFX _returnvalue_2)
              (Variables|Default|SetTracerTrigger false))))
        (:Is%20Not%20Valid
          (goto _label_2)))
      (Variables|Default|SetTracerTrigger (not (Variables|Default|GetTracerTrigger)))
      (Class|NiagaraDataInterfaceArrayFunctionLibrary|SetNiagaraArrayVector (Variables|Default|GetNS_TracerFX) "User.ImpactPositions" (Variables|Default|GetImpact%20Positions))
      (Class|NiagaraComponent|SetVariableBool (Variables|Default|GetNS_TracerFX) "User.Trigger" (Variables|Default|GetTracerTrigger)))
    (:then_2
      (Utilities|FlowControl|RetriggerableDelay 3.0 :!label _label_3)
      (if (or (Utilities|IsValid (Variables|Default|GetNS_MuzzleFlash)) (Utilities|IsValid (Variables|Default|GetNS_TracerFX)))
        (goto _label_3)
        (else
          (Actor|DestroyActor))))))

(fn ConstructionScript)