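; Weapon impact effects actor that turns a shot's hit positions, normals and surface types into Niagara impact effects.
; WeaponFired sorts hits by surface, then feeds concrete and glass batches into one reused system each via Niagara arrays, though glass receives concrete normals.
; A retriggerable delay loop destroys the actor once its systems are gone.
; Metal, body spark and damage number logic is present but unconnected.
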(event Custom|WeaponFired
  (params (ImpactPositions :type Array%20of%20Vectors) (ImpactNormals :type Array%20of%20Vectors) (ImpactSurfaces :type Array%20of%20EPhysicalSurface%20Enums :default "SurfaceType_Default") (MuzzlePosition :type Vector))
  (bind _glassimpacts (Variables|Default|GetGlassImpacts))
  (bind _concreteimpacts (Variables|Default|GetConcreteImpacts))
  (bind _output (Utilities|Array|Get(acopy) _glassimpacts))
  (bind _output_2 (Utilities|Array|Get(acopy) _concreteimpacts))
  (Variables|Default|SetImpact%20Positions ImpactPositions)
  (Variables|Default|SetImpact%20Normals ImpactNormals)
  (Variables|Default|SetImpact%20Surfaces ImpactSurfaces)
  (Variables|Default|SetMuzzle%20Position MuzzlePosition)
  (CallFunction|SplitArraysbySurface)
  (Utilities|FlowControl|Sequence
    (:then_0
      (if (Utilities|Array|IsNotEmpty (Variables|Default|GetConcreteImpacts))
        (Utilities|IsValid (Variables|Default|GetNS_Concrete)
          (:Is%20Valid
            (if (Components|Activation|IsActive (Variables|Default|GetNS_Concrete))
              (Transformation|SetWorldLocation (Variables|Default|GetNS_Concrete) _output_2 false false)
              (else
                (bind _returnvalue (Niagara|SpawnSystematLocation "/Game/Effects/Particles/Impacts/NS_ImpactConcrete.NS_ImpactConcrete" _output_2 :!label _label))
                (Variables|Default|SetNS_Concrete _returnvalue))))
          (:Is%20Not%20Valid
            (goto _label)))
        (Class|NiagaraDataInterfaceArrayFunctionLibrary|SetNiagaraArrayPosition (Variables|Default|GetNS_Concrete) "User.ImpactPositions" (Variables|Default|GetConcreteImpacts))
        (Class|NiagaraDataInterfaceArrayFunctionLibrary|SetNiagaraArrayVector (Variables|Default|GetNS_Concrete) "User.ImpactNormals" (Variables|Default|GetConcreteNormals))
        (Class|NiagaraComponent|SetVariableInt (Variables|Default|GetNS_Concrete) "User.NumberOfHits" (Utilities|Array|Length (Variables|Default|GetConcreteImpacts)))
        (Class|NiagaraComponent|SetVariablePosition (Variables|Default|GetNS_Concrete) "User.MuzzlePosition" (Variables|Default|GetMuzzle%20Position))
        (Components|Activation|Activate (Variables|Default|GetNS_Concrete) false)))
    (:then_1
      (if (Utilities|Array|IsNotEmpty (Variables|Default|GetGlassImpacts))
        (Utilities|IsValid (Variables|Default|GetNS_Glass)
          (:Is%20Valid
            (if (Components|Activation|IsActive (Variables|Default|GetNS_Glass))
              (Transformation|SetWorldLocation (Variables|Default|GetNS_Glass) _output false false)
              (else
                (bind _returnvalue_2 (Niagara|SpawnSystematLocation "/Game/Effects/Particles/Impacts/NS_ImpactGlass.NS_ImpactGlass" _output :!label _label_2))
                (Variables|Default|SetNS_Glass _returnvalue_2))))
          (:Is%20Not%20Valid
            (goto _label_2)))
        (Class|NiagaraDataInterfaceArrayFunctionLibrary|SetNiagaraArrayPosition (Variables|Default|GetNS_Glass) "User.ImpactPositions" (Variables|Default|GetGlassImpacts))
        (Class|NiagaraDataInterfaceArrayFunctionLibrary|SetNiagaraArrayVector (Variables|Default|GetNS_Glass) "User.ImpactNormals" (Variables|Default|GetConcreteNormals))
        (Class|NiagaraComponent|SetVariableInt (Variables|Default|GetNS_Glass) "User.NumberOfHits" (Utilities|Array|Length (Variables|Default|GetGlassImpacts)))
        (Class|NiagaraComponent|SetVariablePosition (Variables|Default|GetNS_Glass) "User.MuzzlePosition" (Variables|Default|GetMuzzle%20Position))
        (Components|Activation|Activate (Variables|Default|GetNS_Glass) false)))
    (:then_3
      (Utilities|Array|Clear (Variables|Default|GetBodyImpacts))
      (Utilities|Array|Clear (Variables|Default|GetBodyNormals))
      (Utilities|Array|Clear (Variables|Default|GetConcreteImpacts))
      (Utilities|Array|Clear (Variables|Default|GetConcreteNormals))
      (Utilities|Array|Clear (Variables|Default|GetGlassImpacts))
      (Utilities|Array|Clear (Variables|Default|GetGlassNormals))
      (Utilities|Array|Clear (Variables|Default|GetMetalImpact))
      (Utilities|Array|Clear (Variables|Default|GetMetalNormals))
      (Utilities|Array|Clear (Variables|Default|GetDamageInfo)))
    (:then_4
      (Utilities|FlowControl|RetriggerableDelay 3.0 :!label _label_3)
      (if (Math|Boolean|ORBoolean (Utilities|IsValid (Variables|Default|GetNS_Concrete)) (Utilities|IsValid (Variables|Default|GetNS_Glass)) (Utilities|IsValid (Variables|Default|GetNS_DamageNumbers)))
        (goto _label_3)
        (else
          (Actor|DestroyActor))))))

(fn ConstructionScript)

(fn SplitArraysbySurface
  (for (_array_element _array_index) (Variables|Default|GetImpact%20Surfaces)
    (if (not (Utilities|Enum|Equal(Enum) _array_element "SurfaceType_Default"))
      (if (Utilities|Enum|Equal(Enum) _array_element "SurfaceType5")
        (Utilities|Array|Add (Variables|Default|GetBodyImpacts) (Utilities|Array|Get(acopy) (Variables|Default|GetImpact%20Positions) _array_index))
        (Utilities|Array|Add (Variables|Default|GetBodyNormals) (Utilities|Array|Get(acopy) (Variables|Default|GetImpact%20Normals) _array_index))
        (elif (Utilities|Enum|Equal(Enum) _array_element "SurfaceType3")
          (Utilities|Array|Add (Variables|Default|GetConcreteImpacts) (Utilities|Array|Get(acopy) (Variables|Default|GetImpact%20Positions) _array_index))
          (Utilities|Array|Add (Variables|Default|GetConcreteNormals) (Utilities|Array|Get(acopy) (Variables|Default|GetImpact%20Normals) _array_index))
          (elif (Utilities|Enum|Equal(Enum) _array_element "SurfaceType6")
            (Utilities|Array|Add (Variables|Default|GetGlassImpacts) (Utilities|Array|Get(acopy) (Variables|Default|GetImpact%20Positions) _array_index))
            (Utilities|Array|Add (Variables|Default|GetGlassNormals) (Utilities|Array|Get(acopy) (Variables|Default|GetImpact%20Normals) _array_index)))))))
  (return))