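; Portal entrance actor for the Arabic West environment that teleports characters overlapping its box to a portal end point.
; For the local player it also adjusts scene lighting, picking one of three light sources by dark, bright or normal map flags.
; On rainy maps it toggles the player pawn's Niagara effect.
; The construction script pushes exposed scale and colour values into the teleport Niagara VFX.
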(event OnComponentBeginOverlap(Box)
  (params (OverlappedComponent :type Primitive%20Component%20Object%20Reference) (OtherActor :type Actor%20Object%20Reference) (OtherComp :type Primitive%20Component%20Object%20Reference) (OtherBodyIndex :type Integer) (bFromSweep :type Boolean) (SweepResult :type Hit%20Result%20Structure%20%28by%20ref%29))
  (bind _ascharacter_prototype_2_base (Utilities|Casting|CastToCharacter_Prototype_2_Base OtherActor))
  (Default|TeleportChar _ascharacter_prototype_2_base (Variables|Default|GetPortal_EndPoint))
  (if (== OtherActor (Game|GetPlayerCharacter 0))
    (Utilities|FlowControl|Sequence
      (:then_0
        (if (Variables|Default|GetDarkMap)
          (Rendering|Components|Light|SetIntensity (Variables|/Script/Engine.Light|GetLightComponent (Variables|Default|GetLightSource_Dark)) 0.9)
          (elif (Variables|Default|GetBrightMap)
            (Rendering|Components|Light|SetIntensity (Variables|/Script/Engine.Light|GetLightComponent (Variables|Default|GetLightSource_Bright)) 3.7)
            (else
              (Rendering|Components|Light|SetIntensity (Variables|/Script/Engine.Light|GetLightComponent (Variables|Default|GetLightSource_Normal)) 3.0)))))
      (:then_1
        (if (Variables|Default|GetRainingMap)
          (bind _ascharacter_prototype_2_base_2 (Utilities|Casting|CastToCharacter_Prototype_2_Base (Pawn|GetControlledPawn (Game|GetPlayerController 0))))
          (Components|Activation|ToggleActive (Variables|/Game/Assets/Character/Character_Prototype_2_Base.Character_Prototype_2_Base_C|GetNiagara _ascharacter_prototype_2_base_2)))))))

(event EventBeginPlay)

(fn ConstructionScript
  (Utilities|FlowControl|Sequence
    (:then_0
      (Niagara|SetNiagaraVariable(Float) (Variables|Default|GetNS_Teleport) "Scale" (Variables|Default|GetVFX_Scale)))
    (:then_1
      (Niagara|SetNiagaraVariable(LinearColor) (Variables|Default|GetNS_Teleport) "Color01" (Variables|Default|GetVFX_Colour)))))