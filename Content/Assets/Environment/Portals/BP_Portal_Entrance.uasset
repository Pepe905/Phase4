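; Portal entrance that teleports the player to a linked end point and adjusts the lighting for the destination.
; Any overlap with its Box moves player pawn 0 to PortalEndPoint's location, with no check on which actor entered.
; The DarkMap and BrightMap flags then pick the dark, bright or normal light source and set its intensity, leaving the other two untouched.
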(event OnComponentBeginOverlap(Box)
  (params (OverlappedComponent :type Primitive%20Component%20Object%20Reference) (OtherActor :type Actor%20Object%20Reference) (OtherComp :type Primitive%20Component%20Object%20Reference) (OtherBodyIndex :type Integer) (bFromSweep :type Boolean) (SweepResult :type Hit%20Result%20Structure%20%28by%20ref%29))
  (Transformation|SetActorLocation (Game|Player|GetPlayerPawn 0) (Transformation|GetActorLocation (Variables|Default|GetPortal_EndPoint)) false false)
  (if (Variables|Default|GetDarkMap)
    (Rendering|Components|Light|SetIntensity (Variables|/Script/Engine.Light|GetLightComponent (Variables|Default|GetLightSource_Dark)) 1.0)
    (elif (Variables|Default|GetBrightMap)
      (Rendering|Components|Light|SetIntensity (Variables|/Script/Engine.Light|GetLightComponent (Variables|Default|GetLightSource_Bright)) 7.0)
      (else
        (Rendering|Components|Light|SetIntensity (Variables|/Script/Engine.Light|GetLightComponent (Variables|Default|GetLightSource_Normal)) 3.0)))))

(event EventBeginPlay)

(event Collision|EventActorBeginOverlap
  (params (OtherActor :type Actor%20Object%20Reference)))

(event EventTick
  (params (DeltaSeconds :type Float%20%28single-precision%29)))

(fn ConstructionScript)