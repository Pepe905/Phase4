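; Interactable chest actor that rewards player 0 with XP, a shield and full health.
; Its collider shows a newly created open-prompt widget on player overlap and hides it on exit.
; Interact switches on authority, reaching the Mc open event through the Svr event or directly on remote.
; That event runs once, playing animation, Niagara effect and sound, then after a delay grants rewards and destroys the chest.
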(event OnComponentBeginOverlap(ChestCollider)
  (params (OverlappedComponent :type Primitive%20Component%20Object%20Reference) (OtherActor :type Actor%20Object%20Reference) (OtherComp :type Primitive%20Component%20Object%20Reference) (OtherBodyIndex :type Integer) (bFromSweep :type Boolean) (SweepResult :type Hit%20Result%20Structure%20%28by%20ref%29))
  (if (== OtherActor (Game|GetPlayerCharacter 0))
    (bind _returnvalue (UserInterface|CreateWidget "/Game/UI/HUD/ChestOpen_Widget.ChestOpen_Widget_C"))
    (bind _output_get (Variables|Default|SetNewVar_0 _returnvalue))
    (UserInterface|Viewport|AddtoViewport _output_get 0)
    (Widget|SetVisibility _output_get "Visible")))

(event OnComponentEndOverlap(ChestCollider)
  (params (OverlappedComponent :type Primitive%20Component%20Object%20Reference) (OtherActor :type Actor%20Object%20Reference) (OtherComp :type Primitive%20Component%20Object%20Reference) (OtherBodyIndex :type Integer))
  (Widget|SetVisibility (stale OnComponentBeginOverlap(ChestCollider) _returnvalue) "Hidden"))

(event Custom|Mc_OpenCHest
  (bind _returnvalue (Game|GetPlayerCharacter 0))
  (Utilities|FlowControl|DoOnce false
    (:Completed
      (Components|Animation|PlayAnimation (Variables|Default|GetSkeletalMesh) "/Game/Assets/Environment/Chest/Chest_Anim_Armature_A_Open.Chest_Anim_Armature_A_Open" false)
      (AddComponent|AddNiagaraComponent false (Math|Transform|MakeTransform "0, 0,120.000000" "0, 0, 0" "3.000000,3.000000,3.000000"))
      (Audio|PlaySound2D "/Game/Assets/Environment/Chest/Chest_Open.Chest_Open" 1.0 1.0 0.0 0 0)
      (Utilities|FlowControl|Delay 4.0)
      (bind _ascharacter_prototype_2 (Utilities|Casting|CastToCharacter_Prototype_2_Base _returnvalue))
      (if (== _ascharacter_prototype_2 _returnvalue)
        (Default|AddBasicXPCharacter _ascharacter_prototype_2 50)
        (Default|AddPlayerShield _ascharacter_prototype_2)
        (bind _output_get (Variables|/Game/Assets/Character/Character_Prototype_2_Base.Character_Prototype_2_Base_C|SetHealth _ascharacter_prototype_2 (Variables|/Game/Assets/Character/Character_Prototype_2_Base.Character_Prototype_2_Base_C|GetMaxHealth _ascharacter_prototype_2)))
        (Default|ClientUpdateHUDHealth _ascharacter_prototype_2 _output_get false)
        (Actor|DestroyActor)))))

(event Custom|Svr_OpenChest
  (CallFunction|McOpenCHest))

(event EventInteract
  (Networking|SwitchHasAuthority
    (:Authority
      (CallFunction|SvrOpenChest))
    (:Remote
      (CallFunction|McOpenCHest))))

(fn ConstructionScript)