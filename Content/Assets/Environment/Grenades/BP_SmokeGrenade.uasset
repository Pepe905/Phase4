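; BP_SmokeGrenade is a thrown smoke grenade actor that releases a smoke cloud after a fuse delay.
; On BeginPlay it launches its mesh with an impulse along the actor's forward vector.
; After a short delay it spawns a scaled-up NS_Smoke Niagara system at its Scene component's location, then later destroys that effect and itself.
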(event EventBeginPlay
  (bind _scene (Variables|Default|GetScene))
  (Physics|AddImpulse (Variables|Default|GetSmokeGrenade) (* (Math|Rotator|GetRotationXVector (Transformation|GetActorRotation)) "1000.000000,1000.000000,1000.000000") "None" false)
  (Utilities|FlowControl|Delay 4.0)
  (bind _output_get (Variables|Default|SetNewVar (Transformation|GetWorldLocation _scene)))
  (bind _returnvalue (Niagara|SpawnSystematLocation "/Game/Assets/Environment/Grenades/NS_Smoke.NS_Smoke" _output_get (Transformation|GetWorldRotation _scene) "6.000000,6.000000,6.000000"))
  (Utilities|FlowControl|Delay 2e+01)
  (Components|DestroyComponent _returnvalue)
  (Actor|DestroyActor))

(fn ConstructionScript)