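; BP_FlashBang is a thrown flashbang grenade that triggers a flash effect on the first player's character.
; On BeginPlay it launches its physics component along the actor's forward vector with a random spin and immediately plays an explosion sound.
; After a fuse delay it calls Flashbang on that character, passing their distance and the grenade's world location as FacingAngle, leaving the effect to the character.
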(event EventBeginPlay
  (bind _flashbang (Variables|Default|GetFlashBang))
  (bind _returnvalue (Transformation|GetWorldLocation _flashbang))
  (bind _ascharacter_prototype_2_base (Utilities|Casting|CastToCharacter_Prototype_2_Base (Game|Player|GetPlayerPawn 0)))
  (Physics|AddImpulse _flashbang (* (Math|Rotator|GetRotationXVector (Transformation|GetActorRotation)) "1000.000000,1000.000000,1000.000000") "None" true)
  (Class|PrimitiveComponent|AddAngularImpulseinDegrees _flashbang (* (Math|Random|RandomUnitVector) 3.5e+02) "None" false)
  (Audio|PlaySoundatLocation "/Game/StarterContent/Audio/Explosion01.Explosion01" _returnvalue "0, 0, 0" 1.0 1.0 0.0 0 0 0 0)
  (Utilities|FlowControl|Delay 3.0)
  (Default|Flashbang _ascharacter_prototype_2_base (Transformation|GetDistanceTo _ascharacter_prototype_2_base) _returnvalue))

(fn ConstructionScript)